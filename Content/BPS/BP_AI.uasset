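; AI pawn that moves to a perceived player and spawns a BP_Enemy with an explosion effect on arrival.
; Perception updates store any BP_TPSPlayer as Target and trigger a move to that player's location at that moment.
; A successful move spawns the enemy and emitter at the pawn's position, while a failed one prints "no path".
; The pawn is not destroyed afterward, as its DestroyActor node is unconnected.
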(event OnPerceptionUpdated(AIPerception)
  (params (UpdatedActors :type Array%20of%20Actor%20Object%20References))
  (bind _array_element (Utilities|Array|ForEachLoopwithBreak UpdatedActors)
    (:LoopBody
      (bind _asbp_tpsplayer (Utilities|Casting|CastToBP_TPSPlayer _array_element))
      (Variables|Default|SetTarget _asbp_tpsplayer)
      (CallFunction|Move))))

(event OnTargetPerceptionUpdated(AIPerception)
  (params (Actor :type Actor%20Object%20Reference) (Stimulus :type AI%20Stimulus%20Structure)))

(event Custom|move
  (bind _returnvalue (Transformation|GetActorLocation))
  (bind _target (Variables|Default|GetTarget))
  (Utilities|IsValid _target
    (:Is%20Valid
      (AI|AIMoveTo self (Transformation|GetActorLocation _target) 0 2e+01 false
        (:OnSuccess
          (Development|PrintString "finished")
          (Game|SpawnActorfromClass "/Game/BPS/BP_Enemy.BP_Enemy_C" (Math|Conversions|ToTransform(Vector) _returnvalue) "Undefined" 0 0)
          (Effects|SpawnEmitteratLocation "/Game/StarterContent/Particles/P_Explosion.P_Explosion" _returnvalue "0, 0, 0" "5.000000,5.000000,5.000000"))
        (:OnFail
          (Development|PrintString "no path"))))))

(event EventBeginPlay)

(event Collision|EventActorBeginOverlap
  (params (OtherActor :type Actor%20Object%20Reference)))

(event EventTick
  (params (DeltaSeconds :type Float%20%28single-precision%29)))

(fn ConstructionScript)