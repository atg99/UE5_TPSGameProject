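; BP_Enemy is an enemy actor with a world-space HP bar widget that turns toward the player's camera.
; BeginPlay passes the actor to its WB_EnemyHP widget as Me, and Tick rotates the widget from the actor-to-camera direction and the actor's up vector.
; An Idle, Move and Attack chase state machine targeting the player pawn is present but disconnected, so it never runs.
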(event EventBeginPlay
  (bind _aswb_enemy_hp (Utilities|Casting|CastToWB_EnemyHP (UserInterface|GetWidget (Variables|Default|GetWidget))))
  (Variables|/Game/BPS/WB_EnemyHP.WB_EnemyHP_C|Setme _aswb_enemy_hp self))

(event Collision|EventActorBeginOverlap
  (params (OtherActor :type Actor%20Object%20Reference)))

(event EventTick
  (params (DeltaSeconds :type Float%20%28single-precision%29))
  (Transformation|SetWorldRotation (Variables|Default|GetWidget) (Math|Rotator|MakeRotfromXZ (- (Transformation|GetActorLocation (Game|GetPlayerCameraManager 0)) (Transformation|GetActorLocation)) (Transformation|GetActorUpVector)) false false))

(fn ConstructionScript)