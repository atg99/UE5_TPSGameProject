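; Third-person shooter player character Blueprint that handles the camera-aimed hit trace for firing.
; CamLinetrace traces from the camera along Visibility, passing the hit flag and a gun-muzzle-to-hit rotation to FireComp so shots converge on the aim point.
; Hits spawn an explosion effect and push physics-simulating components with mass-scaled force.
; BeginPlay only creates the hit widget; CallHit is empty, and camera shake, fade and crouch nodes are unwired.
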(event EventBeginPlay
  (UserInterface|CreateWidget "/Game/BPS/Widget/WB_hit.WB_hit_C"))

(event Collision|EventActorBeginOverlap
  (params (OtherActor :type Actor%20Object%20Reference)))

(event EventTick
  (params (DeltaSeconds :type Float%20%28single-precision%29)))

(event EventCamLinetrace
  (bind _cam (Variables|Default|Getcam))
  (bind _firecomp (Variables|Default|GetfireComp))
  (bind _returnvalue (Transformation|GetWorldLocation _cam))
  (bind (_outhit _returnvalue_2) (Collision|LineTraceByChannel _returnvalue (+ (* (Math|Vector|GetForwardVector _cam) 1e+04) _returnvalue) "TraceTypeQuery1" false (Utilities|Array|MakeArray self 0) "ForOneFrame"))
  (Variables|/Script/TPS_GameProject.PlayerFireComp|SetisHit _firecomp _returnvalue_2)
  (if _returnvalue_2
    (bind _output_get (Variables|Default|SetHitLoc (.Location (Collision|BreakHitResult _outhit))))
    (Variables|/Script/TPS_GameProject.PlayerFireComp|SetspawnRot _firecomp (Math|Conversions|RotationFromXVector (- _output_get (Transformation|GetSocketLocation (Variables|Default|GetgunMeshComp) "FirePosition"))))
    (Effects|SpawnEmitteratLocation "/Game/StarterContent/Particles/P_Explosion.P_Explosion" (.ImpactPoint (Collision|BreakHitResult _outhit)))
    (Utilities|IsValid (.HitComponent (Collision|BreakHitResult _outhit))
      (:Is%20Valid
        (if (Physics|IsSimulatingPhysics (.HitComponent (Collision|BreakHitResult _outhit)) "None")
          (Physics|AddForce (.HitComponent (Collision|BreakHitResult _outhit)) (* (Math|Vector|Normalize (- (.TraceEnd (Collision|BreakHitResult _outhit)) (.TraceStart (Collision|BreakHitResult _outhit)))) 1e+06 (Physics|GetMass (.HitComponent (Collision|BreakHitResult _outhit)))) "None" false))))))

(event EventCallHit)

(event Input|ActionEvents|InputActionCrouch
  (params (Key :type Key%20Structure :default "None")))

(fn ConstructionScript)